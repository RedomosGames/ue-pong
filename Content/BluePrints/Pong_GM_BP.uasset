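; Game mode Blueprint for a Pong game that tracks player and AI scores and ends the match at a score limit.
; IncreamentScore adds a point to either side while a match is in progress and calls CallUpdateScore to broadcast both totals.
; Reaching the limit calls CallGameOver with the winner, stops scoring, and reopens the main menu level after a short delay.
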(event Custom|IncreamentScore
  (params (didPlayerScore? :type Boolean))
  (bind _scorelimit (Variables|Default|GetScoreLimit))
  (if (Variables|Default|GetisInProgress?)
    (if didPlayerScore?
      (bind _result (Math|Integer|IncrementInt (Variables|Default|GetPlayer%20Score))
        (:%20%20
          (Default|CallUpdateScore (Variables|Default|GetPlayer%20Score) (Variables|Default|GetAIScore))
          (if (>= _result _scorelimit)
            (Default|CallGameOver true)
            (Variables|Default|SetisInProgress? false :!label _label)
            (Utilities|FlowControl|Delay 3.0)
            (Game|OpenLevel(byObjectReference) "/Game/Maps/MainMenu_LVL.MainMenu_LVL"))))
      (else
        (bind _result_2 (Math|Integer|IncrementInt (Variables|Default|GetAIScore))
          (:%20%20
            (Default|CallUpdateScore (Variables|Default|GetPlayer%20Score) (Variables|Default|GetAIScore))
            (if (>= _result_2 _scorelimit)
              (Default|CallGameOver false)
              (goto _label))))))))

(fn ConstructionScript)