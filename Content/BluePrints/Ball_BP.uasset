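; Ball actor that bounces around the level at a steadily rising speed and can respawn at its start point.
; Tick moves it along Direction with a swept offset; each blocking hit reflects the direction off the impact normal and increases BallSpeed.
; BeginPlay stores the start location, and both it and Reswpan pick a random normalized direction with a wider Y range than X.
; Respawning leaves BallSpeed unchanged.
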(event Custom|Change%20Direction
  (Variables|Default|SetDirection (Math|Vector|Normalize (Math|Vector|MakeVector (Math|Random|RandomFloatinRange -0.5 0.5) (Math|Random|RandomFloatinRange -1.0 1.0) 0.0))))

(event Custom|Reswpan
  (CallFunction|ChangeDirection)
  (Transformation|SetActorLocation (Variables|Default|GetStartingLocation) false false))

(event EventBeginPlay
  (CallFunction|ChangeDirection)
  (Variables|Default|SetStartingLocation (Transformation|GetActorLocation)))

(event EventTick
  (params (DeltaSeconds :type Float%20%28single-precision%29))
  (bind _sweephitresult (Transformation|AddActorWorldOffset (* DeltaSeconds (Variables|Default|GetBallSpeed) (Variables|Default|GetDirection)) true))
  (if (.bblockinghit _sweephitresult)
    (Variables|Default|SetDirection (Math|Vector|Normalize (Math|Vector|GetReflectionVector (Variables|Default|GetDirection) (.impactnormal _sweephitresult))))
    (Variables|Default|SetBallSpeed (+ (Variables|Default|GetBallSpeed) 2e+01))))

(fn ConstructionScript)